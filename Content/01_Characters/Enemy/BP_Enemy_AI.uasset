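; Enemy AI character Blueprint with state and status components, a world health label and generic team ID 2.
; BeginPlay spawns hit effect actors and initializes stats, while Tick refreshes the label's health and render scale.
; SendDamage stores hit data and sets Hitted state, whose change event applies damage and checks health.
; Death disables capsule collision, sets the behavior tree component to dead mode, ragdolls the mesh and disables movement.
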(event Custom|OnStateTypeChanged
  (params (InPrevType :type EStateType%20Enum :default "NewEnumerator0") (InNewType :type EStateType%20Enum :default "NewEnumerator0"))
  (switch Utilities|FlowControl|Switch|SwitchonEStateType InNewType
    (:NewEnumerator5
      (CallFunction|OnHitted))
    (:NewEnumerator7
      (CallFunction|OnDead))))

(event EventBeginPlay
  (bind _statuscomponent (Variables|Default|GetStatusComponent))
  (Utilities|FlowControl|Sequence
    (:then_0
      (bind _returnvalue (Game|SpawnActorfromClass "/Game/02_Components/WeaponComponent/Hitted/BP_HittedEffect.BP_HittedEffect_C" (Math|Transform|MakeTransform "0, 0, 0") "Undefined" self 0))
      (Variables|Hitted|SetHittedEffect _returnvalue)
      (bind _returnvalue_2 (Game|SpawnActorfromClass "/Game/06_Effects/TargetingEffect/BP_TargetHittedEffect.BP_TargetHittedEffect_C" (Math|Transform|MakeTransform "0, 0, 0") "Undefined" self 0))
      (Variables|Hitted|SetTargetHittedEffect _returnvalue_2))
    (:then_1
      (EventDispatchers|BindEventtoOnStateTypeChanged (Variables|Default|GetStateComponent) (EventDispatchers|CreateEvent :!event Custom|OnStateTypeChanged))
      (Default|InitStatus (Variables|Default|GetStatusComponent) 1e+02 1e+02))
    (:then_2
      (bind _aswb_label_health (Utilities|Casting|CastToWB_LabelHealth (UserInterface|GetUserWidgetObject (Variables|Default|GetLabel))))
      (Variables|Label|SetLabelClass _aswb_label_health)
      (Default|UpdateName (Variables|Label|GetLabelClass) (Utilities|GetDisplayName self))
      (Default|UpdateHealth (Variables|Label|GetLabelClass) (Default|GetCurrentHealth _statuscomponent) (Default|GetMaxHealth _statuscomponent)))
    (:then_3
      (Utilities|Struct|SetmembersinGenericTeamId (Utilities|Struct|MakeGenericTeamId 2)))))

(event EventSendDamage
  (params (InAttacker :type Character%20Object%20Reference) (InWeapon :type Actor%20Object%20Reference) (InHitData :type F%20Hit%20Data%20Structure) (InHitLocation :type Vector :default "0, 0, 0"))
  (Variables|Hitted|SetAttacker InAttacker)
  (Variables|Hitted|SetAttackingWeapon InWeapon)
  (Variables|Hitted|SetHittedData InHitData)
  (Variables|Hitted|SetHittedLocation InHitLocation)
  (Default|SetHittedMode (Variables|Default|GetStateComponent)))

(event EventTick
  (params (DeltaSeconds :type Float%20%28single-precision%29))
  (bind _statuscomponent (Variables|Default|GetStatusComponent))
  (Utilities|FlowControl|Sequence
    (:then_0
      (bind _labelclass (Variables|Label|GetLabelClass)
        (:then
          (Default|UpdateHealth _labelclass (Default|GetCurrentHealth _statuscomponent) (Default|GetMaxHealth _statuscomponent))
          (CallFunction|UpdateLabelRenderScale self (Variables|Label|GetLabelClass) (Variables|Label|GetLabelViewDistance)))
        (:else)))))

(event EventEndHitted
  (Default|EndGlow (Variables|Hitted|GetHittedEffect)))

(fn ConstructionScript)

(fn OnHitted
  (CallFunction|ApplyDamage true self (Variables|Hitted|GetAttacker) (Variables|Hitted|GetHittedLocation) (Variables|Hitted|GetHittedData) (Variables|Hitted|GetHittedEffect))
  (bind _outdead (Default|CheckHealth (Variables|Default|GetStatusComponent) (.Damage (Utilities|Struct|BreakFHitData (Variables|Hitted|GetHittedData)))))
  (if _outdead
    (Collision|SetCollisionEnabled (Variables|Collision|GetCapsuleComponent) "NoCollision")
    (Default|SetDeadMode (Variables|Default|GetStateComponent))))

(fn OnDead
  (Default|SetDeadMode (Variables|Default|GetBehaviorTreeComponent))
  (Class|SkeletalMeshComponent|SetAllBodiesSimulatePhysics (Variables|Character|GetMesh) true)
  (Physics|SetSimulatePhysics (Variables|Character|GetMesh) true)
  (Class|PrimitiveComponent|WakeAllRigidBodies (Variables|Character|GetMesh))
  (Class|SkeletalMeshComponent|SetEnablePhysicsBlending (Variables|Character|GetMesh) true)
  (Pawn|Components|CharacterMovement|DisableMovement (Variables|Character|GetCharacterMovement)))