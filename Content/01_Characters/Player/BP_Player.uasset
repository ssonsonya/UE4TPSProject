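; Player character Blueprint that routes input to components for movement, stamina, weapons, item pickup and parkour, and creates the HUD.
; Transform toggles Normal and Hero modes, swapping stats and weapon sets, with a material-parameter-collection transition effect.
; Incoming damage is stored, then applied through StateComponent's state-change event, switching to Dead on a health check.
; Tick tracks idle time, interpolates camera zoom and toggles control rotation; looping timers drain and recharge stamina.
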(event Custom|OnStateTypeChanged
  (params (InPrevType :type EStateType%20Enum :default "NewEnumerator0") (InNewType :type EStateType%20Enum :default "NewEnumerator0"))
  (switch Utilities|FlowControl|Switch|SwitchonEStateType InNewType
    (:NewEnumerator5
      (CallFunction|OnHitted))
    (:NewEnumerator7
      (CallFunction|OnDead))))

(event EventTick
  (params (DeltaSeconds :type Float%20%28single-precision%29))
  (Utilities|FlowControl|Sequence
    (:then_0
      (CallFunction|CheckIdle DeltaSeconds))
    (:then_1
      (CallFunction|ApplyZoom))
    (:then_2
      (if (Math|Float|NearlyEqual(Float) (Math|Vector|VectorLength (Transformation|GetVelocity)) 0.0 1e-06)
        (if (Variables|Weapon|GetAiming)
          (Default|EnableControlRotation (Variables|Move|GetMoveComponent))
          (else
            (Default|DisableControlRotation (Variables|Move|GetMoveComponent))))
        (else
          (Default|EnableControlRotation (Variables|Move|GetMoveComponent)))))))

(event EventSendDamage
  (params (InAttacker :type Character%20Object%20Reference) (InWeapon :type Actor%20Object%20Reference) (InHitData :type F%20Hit%20Data%20Structure) (InHitLocation :type Vector :default "0, 0, 0"))
  (Variables|Hitted|SetAttacker InAttacker)
  (Variables|Hitted|SetAttackingWeapon InWeapon)
  (Variables|Hitted|SetHittedData InHitData)
  (Variables|Hitted|SetHittedLocation InHitLocation)
  (Default|SetHittedMode (Variables|디폴트|GetStateComponent)))

(event EventBeginPlay
  (bind _transformcomponent (Variables|Stats|GetTransformComponent))
  (Utilities|FlowControl|Sequence
    (:then_0
      ;[1 1 1] HUD
      (bind _returnvalue (UserInterface|CreateWidget "/Game/03_Widgets/WB_PlayerHUD.WB_PlayerHUD_C"))
      (bind _output_get (Variables|UI|SetPlayerHUD _returnvalue))
      (UserInterface|Viewport|AddtoViewport _output_get 0))
    (:then_1
      ;[1 1 1] Initialize Player
      ;;[1 1 1] Init Current Stats Set
      (bind _output_get_2 (Variables|Stats|SetCurrentStats (Utilities|Array|Get(acopy) (Variables|/Game/02_Components/TransformComponent/TransformComponent.TransformComponent_C|GetChracterMode _transformcomponent))))
      (Default|SetCharacterMode _transformcomponent _output_get_2)
      ;;[1 1 1] Init TargetArmLength
      (Variables|Zoom|SetZooming (Variables|/Script/Engine.SpringArmComponent|GetTargetArmLength (Variables|Default|GetSpringArm)))
      ;;[1 1 1] Init Status
      (Default|InitStatus (Variables|Default|GetStatusComponent) 1e+02 1e+02))
    (:then_2
      ;[1 1 1] StateComp
      (EventDispatchers|BindEventtoOnStateTypeChanged (Variables|디폴트|GetStateComponent) (EventDispatchers|CreateEvent :!event Custom|OnStateTypeChanged))
      (bind _returnvalue_2 (Game|SpawnActorfromClass "/Game/02_Components/WeaponComponent/Hitted/BP_HittedEffect.BP_HittedEffect_C" (Math|Transform|MakeTransform "0, 0, 0") "Undefined" self 0))
      (Variables|Hitted|SetHittedEffect _returnvalue_2))))

(event EventEndHitted
  (Default|EndGlow (Variables|Hitted|GetHittedEffect)))

(event Input|ActionEvents|InputActionMenu
  (params (Key :type Key%20Structure :default "None"))
  (:Pressed
    (Utilities|FlowControl|FlipFlop
      (:A
        (CallFunction|EnableMouseCursor))
      (:B
        (CallFunction|DisableMouseCursor)))))

(fn ConstructionScript)

(fn CheckIdle
  (params (InDeltaTime :type Float%20%28single-precision%29))
  (bind _weaponcomponent (Variables|Weapon|GetWeaponComponent))
  (bind _weapon (Default|GetWeapon _weaponcomponent))
  (if (> (Variables|Move|GetNoActionTime) 3e+01)
    (CallFunction|ResetNoActionTime)
    (elif (and (<= (Math|Vector|VectorLength (Pawn|Components|CharacterMovement|GetCurrentAcceleration (Variables|Character|GetCharacterMovement))) 0.0) (Default|IsIdleMode (Variables|디폴트|GetStateComponent)))
      (Utilities|IsValid _weapon
        (:Is%20Valid
          (if (or (Default|IsIdleMode (Variables|Weapon|GetWeaponComponent)) (not (Variables|/Game/02_Components/WeaponComponent/WeaponControl.WeaponControl_C|GetInSubAction _weapon)))
            (Variables|Move|SetNoActionTime (+ (Variables|Move|GetNoActionTime) InDeltaTime) :!label _label)))
        (:Is%20Not%20Valid
          (goto _label)))
      (else
        (CallFunction|ResetNoActionTime)))))

(fn GetNoActionTime
  (return (Variables|Move|GetNoActionTime)))

(fn ResetNoActionTime
  (Variables|Move|SetNoActionTime 0.0))

(fn SetWeaponVisibility
  (params (InVisibility :type Boolean))
  (bind _mesh (Variables|Character|GetMesh))
  (if InVisibility
    (Components|SkinnedMesh|UnHideBonebyName _mesh "weapon_l")
    (Components|SkinnedMesh|UnHideBonebyName _mesh "weapon_r")
    (Components|SkinnedMesh|UnHideBonebyName _mesh "grenade")
    (else
      (Components|SkinnedMesh|HideBonebyName _mesh "weapon_l" "PBO_None")
      (Components|SkinnedMesh|HideBonebyName _mesh "weapon_r" "PBO_None")
      (Components|SkinnedMesh|HideBonebyName _mesh "grenade" "PBO_None"))))

(fn OnHitted
  (CallFunction|ApplyDamage false self (Variables|Hitted|GetAttacker) (Variables|Hitted|GetHittedLocation) (Variables|Hitted|GetHittedData) (Variables|Hitted|GetHittedEffect))
  (bind _outdead (Default|CheckHealth (Variables|Default|GetStatusComponent) (.Damage (Utilities|Struct|BreakFHitData (Variables|Hitted|GetHittedData)))))
  (if _outdead
    (Default|SetDeadMode (Variables|디폴트|GetStateComponent))))

(fn OnDead)

(fn EnableMouseCursor
  (Variables|/Script/Engine.PlayerController|SetbShowMouseCursor (Game|GetPlayerController 0) true))

(fn DisableMouseCursor
  (Variables|/Script/Engine.PlayerController|SetbShowMouseCursor (Game|GetPlayerController 0) false))

(event Custom|OnRelaxed
  ;[1 1 1] Stemina Control
  (bind _outrecharged (Default|RechargeStemina (Variables|Default|GetStatusComponent) 1.0))
  (if _outrecharged
    (Utilities|Time|ClearandInvalidateTimerbyHandle (Variables|Move|GetRechargeSteminaHandler))))

(event Custom|OnRun
  ;[1 1 1] Stemina Control
  (bind _outexhust (Default|UseStemina (Variables|Default|GetStatusComponent) 1.0))
  (if _outexhust
    (Default|SetSpeed (Variables|Move|GetMoveComponent) "NewEnumerator0")))

(event Input|ActionEvents|InputActionRun
  (params (Key :type Key%20Structure :default "None"))
  (bind _movecomponent (Variables|Move|GetMoveComponent))
  (bind _outtype (Default|GetSpeedType _movecomponent))
  ;[1 1 1] Run기능
  (:Pressed
    (Utilities|Time|ClearandInvalidateTimerbyHandle (Variables|Move|GetRechargeSteminaHandler))
    (bind _returnvalue (Utilities|Time|SetTimerbyEvent (EventDispatchers|CreateEvent :!event Custom|OnRun) 0.1 true))
    (Variables|Move|SetUseSteminaHandler _returnvalue)
    (bind _result (Math|Integer|IncrementInt (Variables|Move|GetShiftCount))
      (:%20%20
        (if (>= _result 2)
          (Default|SetSpeed (Variables|Move|GetMoveComponent) "NewEnumerator2")
          (else
            (Default|SetSpeed (Variables|Move|GetMoveComponent) "NewEnumerator1"))))))
  (:Released
    (Default|SetSpeed (Variables|Move|GetMoveComponent) "NewEnumerator0")
    (Utilities|FlowControl|Delay 0.5)
    (Variables|Move|SetShiftCount 0)
    (if (or (Utilities|Enum|Equal(Enum) _outtype "NewEnumerator3") (Utilities|Enum|Equal(Enum) _outtype "NewEnumerator0"))
      (Utilities|Time|ClearandInvalidateTimerbyHandle (Variables|Move|GetUseSteminaHandler))
      (bind _returnvalue_2 (Utilities|Time|SetTimerbyEvent (EventDispatchers|CreateEvent :!event Custom|OnRelaxed) 0.1 true 2.0))
      (Variables|Move|SetRechargeSteminaHandler _returnvalue_2))))

(event Input|ActionEvents|InputActionJump
  (params (Key :type Key%20Structure :default "None"))
  ;[1 1 1] Jump기능
  (:Pressed
    (if (AI|Components|NavMovement|IsFalling (Variables|Character|GetCharacterMovement))
      (Variables|Move|SetDoubleJump true)
      (Character|Jump)
      (else
        (Character|Jump))))
  (:Released
    (Character|StopJumping)
    (Variables|Move|SetDoubleJump false)))

(event Input|ActionEvents|InputActionCrouch
  (params (Key :type Key%20Structure :default "None"))
  (bind _aiming (Variables|Weapon|GetAiming))
  ;[1 1 1] Crouch
  (:Pressed
    (Utilities|FlowControl|FlipFlop
      (:A
        (Character|Crouch)
        (if (not _aiming)
          (bind _camlength (Timeline|CrouchCamLength Play)
            (:Update
              (Variables|/Script/Engine.SpringArmComponent|SetTargetArmLength (Variables|Default|GetSpringArm) (Math|Float|Lerp 3e+02 6e+02 _camlength))))))
      (:B
        (Character|UnCrouch)
        (if (not _aiming)
          (Timeline|CrouchCamLength Reverse))))))

(event Input|ActionEvents|InputActionEvade
  (params (Key :type Key%20Structure :default "None"))
  ;[1 1 1] Evade
  (:Pressed
    (if (Default|IsHeroMode (Variables|Stats|GetTransformComponent))
      (bind _output_get (Variables|Move|SetEvade true))
      (Development|PrintString (Utilities|String|ToString(Boolean) _output_get))))
  (:Released
    (bind _output_get_2 (Variables|Move|SetEvade false))
    (Development|PrintString (Utilities|String|ToString(Boolean) _output_get_2))))

(event Input|AxisEvents|InputAxisMoveRight
  (params (AxisValue :type Float%20%28single-precision%29))
  ;[1 1 1] Move
  (if (Default|IsCanMove (Variables|Move|GetMoveComponent))
    (if (not (Utilities|Enum|Equal(Enum) (Default|GetSpeedType (Variables|Move|GetMoveComponent)) "NewEnumerator2"))
      (Pawn|Input|AddMovementInput (Math|Vector|GetRightVector (Math|Rotator|MakeRotator 0.0 0.0 (.yaw (Pawn|GetControlRotation :!class /Script/Engine.Pawn)))) AxisValue true))))

(event Input|AxisEvents|InputAxisMoveForward
  (params (AxisValue :type Float%20%28single-precision%29))
  ;[1 1 1] Move
  (if (Default|IsCanMove (Variables|Move|GetMoveComponent))
    (Pawn|Input|AddMovementInput (Math|Vector|GetForwardVector (Math|Rotator|MakeRotator 0.0 0.0 (.yaw (Pawn|GetControlRotation :!class /Script/Engine.Pawn)))) AxisValue true)))

(event Input|AxisEvents|InputAxisHorizontalLook
  (params (AxisValue :type Float%20%28single-precision%29))
  ;[1 1 1] Look
  (if (not (Default|GetFixedCamera (Variables|Move|GetMoveComponent)))
    (Pawn|Input|AddControllerYawInput AxisValue)))

(event Input|AxisEvents|InputAxisVerticalLook
  (params (AxisValue :type Float%20%28single-precision%29))
  ;[1 1 1] Look
  (if (not (Default|GetFixedCamera (Variables|Move|GetMoveComponent)))
    (Pawn|Input|AddControllerPitchInput AxisValue)))

(event Input|ActionEvents|InputActionTransform
  (params (Key :type Key%20Structure))
  (bind _transformcomponent (Variables|Stats|GetTransformComponent))
  (bind _transformcomponent_2 (Variables|Stats|GetTransformComponent))
  (:Pressed
    (if (Default|IsIdleMode (Variables|디폴트|GetStateComponent))
      ;[1 1 1] HeroMode Transform
      (bind _isa (Utilities|FlowControl|FlipFlop)
        (:A
          ;;[1 1 1] SetModes
          (Default|SetIdleMode (Variables|Weapon|GetWeaponComponent))
          (Default|SetEquipMode (Variables|디폴트|GetStateComponent))
          ;;[1 1 1] Current Stats Set
          (bind _output_get (Variables|Stats|SetCurrentStats (Utilities|Array|Get(acopy) (Variables|/Game/02_Components/TransformComponent/TransformComponent.TransformComponent_C|GetChracterMode _transformcomponent) 1)))
          (Default|SetCharacterMode _transformcomponent _output_get)
          ;;[1 1 1] PostProcessMaterial Transform Effect Application
          (Game|SpawnActorfromClass "/Game/06_Effects/TransitionEffect/PPV_Transform.PPV_Transform_C" (Math|Transform|MakeTransform (Transformation|GetActorLocation)) "Undefined" 0 0)
          (bind _maptransit (Timeline|MapTransit Play)
            (:Update
              (Rendering|Material|SetScalarParameterValue "/Game/06_Effects/TransitionEffect/PC_TransitionData.PC_TransitionData" "Radius" _maptransit :!class /Script/Engine.KismetMaterialLibrary)
              (if _isa
                (Variables|Transform|SetFirstTransform false)))))
        (:B
          ;[1 1 1] Back to NormalMode Transform
          ;;[1 1 1] Initialize Components
          (Default|SetIdleMode (Variables|Weapon|GetWeaponComponent))
          (Default|SetEquipMode (Variables|디폴트|GetStateComponent))
          ;;[1 1 1] Current Stats Set
          (bind _output_get_2 (Variables|Stats|SetCurrentStats (Utilities|Array|Get(acopy) (Variables|/Game/02_Components/TransformComponent/TransformComponent.TransformComponent_C|GetChracterMode _transformcomponent_2))))
          (Default|SetCharacterMode _transformcomponent_2 _output_get_2)
          (Rendering|Material|SetVectorParameterValue "/Game/06_Effects/TransitionEffect/PC_TransitionData.PC_TransitionData" "Location" (Math|Conversions|ToLinearColor(Vector) (Transformation|GetActorLocation)) :!class /Script/Engine.KismetMaterialLibrary)
          (Timeline|MapTransit Reverse))))))

(event Input|ActionEvents|InputActionUnarmed
  (params (Key :type Key%20Structure))
  ;[1 1 1] Unarmed : No item - Normal : MartialArts / Hero : Gun
  (:Pressed
    (if (Default|IsIdleMode (Variables|디폴트|GetStateComponent))
      (Default|SetUnarmedMode (Variables|Weapon|GetWeaponComponent) false))))

(event Input|ActionEvents|InputActionAttack
  (params (Key :type Key%20Structure))
  ;[1 1 1] Attack
  (:Pressed
    (if (Utilities|Enum|Equal(Enum) (Default|GetCurrentType (Variables|Weapon|GetWeaponComponent)) "NewEnumerator0")
      (Default|SetUnarmedMode (Variables|Weapon|GetWeaponComponent) false))
    (Default|DoAction (Variables|Weapon|GetWeaponComponent))))

(event Input|ActionEvents|InputActionWeapon_Throw
  (params (Key :type Key%20Structure))
  (bind _weaponcomponent (Variables|Weapon|GetWeaponComponent))
  ;[1 1 1] Throwable Weapon : Use item - Normal : Brick, Bottle, etc / Hero : Granade
  (:Pressed
    (if (Default|IsIdleMode (Variables|디폴트|GetStateComponent))
      (if (Utilities|Name|Equal(Name) (Default|GetCurrentModeName (Variables|Stats|GetTransformComponent)) "Normal")
        (Default|SetThrowWeaponMode _weaponcomponent true)
        (else
          (Default|SetThrowWeaponMode _weaponcomponent false))))))

(event Input|ActionEvents|InputActionWeapon_Ult
  (params (Key :type Key%20Structure))
  ;[1 1 1] Ultimate Weapon : Use item - Normal : None / Hero : UltGun
  (:Pressed
    (if (Default|IsIdleMode (Variables|디폴트|GetStateComponent))
      (Default|SetUltWeaponMode (Variables|Weapon|GetWeaponComponent)))))

(event Input|ActionEvents|InputActionSubAction
  (params (Key :type Key%20Structure))
  (bind _weaponcomponent (Variables|Weapon|GetWeaponComponent))
  ;[1 1 1] SubAction : Trowable - Aim
  (:Pressed
    (Default|SubActionPressed _weaponcomponent))
  (:Released
    (Default|SubActionReleased _weaponcomponent)))

(event Input|ActionEvents|InputActionWeapon
  (params (Key :type Key%20Structure))
  ;[1 1 1] Weapon : Use item - Normal : BaseballBat / Hero : Knife
  (:Pressed
    (if (Default|IsIdleMode (Variables|디폴트|GetStateComponent))
      (Default|SetWeaponMode (Variables|Weapon|GetWeaponComponent) (Utilities|Name|Equal(Name) (Default|GetCurrentModeName (Variables|Stats|GetTransformComponent)) "Normal")))))

(event Input|ActionEvents|InputActionInteraction
  (params (Key :type Key%20Structure :default "None"))
  (:Pressed
    (for _array_element (Collision|GetOverlappingActors "/Game/02_Components/InventoryComponent/BP_Item.BP_Item_C" :!class /Script/Engine.Actor)
      (bind _asbp_item (Utilities|Casting|CastToBP_Item _array_element))
      (Default|PickUpItem (Variables|Default|GetInventoriyComponent) _asbp_item))))

(event Custom|ApplyZoom
  (if (not (AI|Components|NavMovement|IsCrouching (Variables|Character|GetCharacterMovement)))
    (if (not (Variables|Weapon|GetAiming))
      (if (not (Math|Float|NearlyEqual(Float) (Variables|Zoom|GetZooming) (Variables|/Script/Engine.SpringArmComponent|GetTargetArmLength (Variables|Default|GetSpringArm)) 1e-06))
        (Variables|/Script/Engine.SpringArmComponent|SetTargetArmLength (Variables|Default|GetSpringArm) (Math|Interpolation|FInterpTo (Variables|/Script/Engine.SpringArmComponent|GetTargetArmLength (Variables|Default|GetSpringArm)) (Variables|Zoom|GetZooming) (Utilities|Time|GetWorldDeltaSeconds) (.interpspeed (Variables|Zoom|GetZoomData))))))))

(event Input|AxisEvents|InputAxisZoom
  (params (AxisValue :type Float%20%28single-precision%29))
  (bind _zoomdata (Variables|Zoom|GetZoomData))
  (if (not (AI|Components|NavMovement|IsCrouching (Variables|Character|GetCharacterMovement)))
    (if (not (Variables|Weapon|GetAiming))
      (Variables|Zoom|SetZooming (Math|Float|Clamp(Float) (+ (Variables|Zoom|GetZooming) (* AxisValue (.speed _zoomdata))) (.minrange _zoomdata) (.maxrange _zoomdata))))))

(event EventOnLanded
  (params (Hit :type Hit%20Result%20Structure%20%28by%20ref%29))
  ;[1 1 1] LandedMode
  (Default|DoParkourLandedMode (Variables|Default|GetParkourComponent)))

(event Input|ActionEvents|InputActionParkour
  (params (Key :type Key%20Structure))
  ;[1 1 1] DoParkour
  (:Pressed
    (Default|DoParkour (Variables|Default|GetParkourComponent))))