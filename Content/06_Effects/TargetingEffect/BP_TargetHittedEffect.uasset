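; BP_TargetHittedEffect is an effect actor that overlays a glow on its owning Character, toggled by StartGlow and EndGlow.
; On BeginPlay it hides a PoseableMesh, gives it the owner's skeletal mesh and fills its material slots with the HittedEffect material.
; Each tick it snaps to the owner mesh's world transform and copies its pose, so the duplicate mesh follows the animation.
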(event Custom|EndGlow
  (Rendering|SetVisibility (Variables|Default|GetPoseableMesh) false false))

(event Custom|StartGlow
  (Rendering|SetVisibility (Variables|Default|GetPoseableMesh) true false))

(event EventBeginPlay
  (bind _ascharacter (Utilities|Casting|CastToCharacter (Components|GetOwner)))
  (Variables|Default|SetOwnerCharacter _ascharacter)
  (Rendering|SetVisibility (Variables|Default|GetPoseableMesh) false false)
  (for (_ _array_index) (Rendering|Material|GetMaterials (Variables|/Script/Engine.Character|GetMesh (Variables|Default|GetOwnerCharacter)))
    (Rendering|Material|SetMaterial (Variables|Default|GetPoseableMesh) _array_index (Variables|Default|GetHittedEffect)))
  (Class|SkinnedMeshComponent|SetSkeletalMesh (Variables|Default|GetPoseableMesh) (Variables|/Script/Engine.SkinnedMeshComponent|GetSkeletalMesh (Variables|/Script/Engine.Character|GetMesh (Variables|Default|GetOwnerCharacter))) true))

(event EventTick
  (params (DeltaSeconds :type Float%20%28single-precision%29))
  (Transformation|SetActorTransform (Transformation|GetWorldTransform (Variables|/Script/Engine.Character|GetMesh (Variables|Default|GetOwnerCharacter))))
  (Class|PoseableMeshComponent|CopyPosefromSkeletalComponent (Variables|Default|GetPoseableMesh) (Variables|/Script/Engine.Character|GetMesh (Variables|Default|GetOwnerCharacter))))

(fn ConstructionScript)