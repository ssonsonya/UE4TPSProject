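; Patrol route Blueprint that walks its spline points back and forth in a ping-pong order instead of in one direction.
; It overrides the parent's UpdateIndex, calling it first, then stepping Index up or down according to the InReverse flag.
; At either end of the spline it flips InReverse and moves Index to the neighboring point, so the endpoint is not repeated.
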(event EventBeginPlay
  (|CallParentFunction))

(fn ConstructionScript)

(fn UpdateIndex
  (|CallParentFunction)
  (LocalVariables|SetCount (Spline|GetNumberOfSplinePoints (Variables|Default|GetSpline)))
  (if (Variables|Default|GetInReverse)
    (if (> (Variables|Default|GetIndex) 0)
      (Math|Integer|DecrementInt (Variables|Default|GetIndex)
        (:%20%20
          (return)))
      (else
        (Variables|Default|SetIndex 1)
        (Variables|Default|SetInReverse false)))
    (elif (< (Variables|Default|GetIndex) (- (LocalVariables|GetCount) 1))
      (Math|Integer|IncrementInt (Variables|Default|GetIndex)
        (:%20%20
          (return)))
      (else
        (Variables|Default|SetIndex (- (LocalVariables|GetCount) 2))
        (Variables|Default|SetInReverse true)))))