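; BP_LoopRoute is a patrol spline route variant whose point index loops continuously around the spline.
; It overrides UpdateIndex to call the parent, then increment Index until the last spline point and wrap it back to zero.
; BeginPlay and the construction script only forward to the parent.
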(event EventBeginPlay
  (|CallParentFunction))

(fn ConstructionScript
  (|CallParentFunction))

(fn UpdateIndex
  (|CallParentFunction)
  (LocalVariables|SetCount (Spline|GetNumberOfSplinePoints (Variables|Default|GetSpline)))
  (if (< (Variables|Default|GetIndex) (- (LocalVariables|GetCount) 1))
    (Math|Integer|IncrementInt (Variables|Default|GetIndex)
      (:%20%20
        (return)))
    (else
      (Variables|Default|SetIndex 0)
      (return))))