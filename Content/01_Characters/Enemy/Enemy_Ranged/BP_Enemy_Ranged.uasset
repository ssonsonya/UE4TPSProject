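; Ranged enemy Blueprint that changes its form along with the player's mode.
; On BeginPlay it runs the parent logic, then binds to the mode-changed dispatcher on the controlled BP_Player's TransformComponent.
; Its Transform event takes a hero flag, switches its own TransformComponent between two character modes and rescales the capsule, larger for hero mode and smaller otherwise.
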(event Custom|Transform
  (params (InNowHero :type Boolean))
  (if InNowHero
    (Default|SetCharacterMode (Variables|Default|GetTransformComponent) (Utilities|Array|Get(acopy) (Variables|/Game/02_Components/TransformComponent/TransformComponent.TransformComponent_C|GetChracterMode (Variables|Default|GetTransformComponent)) 1))
    (Transformation|SetWorldScale3D (Variables|Default|GetCapsuleComponent) "1.800000,1.800000,1.800000")
    (else
      (Default|SetCharacterMode (Variables|Default|GetTransformComponent) (Utilities|Array|Get(acopy) (Variables|/Game/02_Components/TransformComponent/TransformComponent.TransformComponent_C|GetChracterMode (Variables|Default|GetTransformComponent))))
      (Transformation|SetWorldScale3D (Variables|Default|GetCapsuleComponent) "1.200000,1.200000,1.200000"))))

(event EventBeginPlay
  (|CallParentFunction)
  (bind _asbp_player (Utilities|Casting|CastToBP_Player (Pawn|GetControlledPawn (Game|GetPlayerController 0))))
  (EventDispatchers|BindEventtoOnPlayerModeChanged (Variables|/Game/01_Characters/Player/BP_Player.BP_Player_C|GetTransformComponent _asbp_player) (EventDispatchers|CreateEvent :!event Custom|Transform)))

(fn ConstructionScript
  (|CallParentFunction))