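; BP_ItemFound is a highlight actor that shows a glow over its owning BP_Item.
; On BeginPlay it copies the owner's static mesh, applies the M_ItemFound material and starts hidden.
; It matches the item mesh's world transform every tick, while StartGlow and EndGlow toggle the duplicate mesh's visibility, leaving the item's own materials untouched.
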(event Custom|EndGlow
  (Rendering|SetVisibility (Variables|Default|GetStaticMesh) false false))

(event Custom|StartGlow
  (Rendering|SetVisibility (Variables|Default|GetStaticMesh) true false))

(event EventBeginPlay
  (bind _staticmesh (Variables|Default|GetStaticMesh))
  (bind _asbp_item (Utilities|Casting|CastToBP_Item (Components|GetOwner)))
  (bind _output_get (Variables|Default|SetOwnerItem _asbp_item))
  (Components|StaticMesh|SetStaticMesh _staticmesh (Variables|/Script/Engine.StaticMeshComponent|GetStaticMesh (Variables|/Game/02_Components/InventoryComponent/BP_Item.BP_Item_C|GetStaticMesh _output_get)))
  (Rendering|Material|SetMaterial _staticmesh 0 "/Game/02_Components/InventoryComponent/M_ItemFound.M_ItemFound")
  (Rendering|SetVisibility _staticmesh false false))

(event EventTick
  (params (DeltaSeconds :type Float%20%28single-precision%29))
  (Transformation|SetActorTransform (Transformation|GetWorldTransform (Variables|/Game/02_Components/InventoryComponent/BP_Item.BP_Item_C|GetStaticMesh (Variables|Default|GetOwnerItem)))))

(fn ConstructionScript)