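; BP_Item is a pickup item that glows when found and removes itself from the world when picked up.
; On BeginPlay it spawns a companion BP_ItemFound actor at its own transform to provide the glow.
; SetItemFound raises a flag that Tick consumes to start the glow and set a short timer, then clears.
; PickUp prints a debug message and destroys both the glow actor and the item.
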(event Custom|PickUp
  (Development|PrintString "ItemPicked")
  (Actor|DestroyActor (Variables|Default|GetFoundGlow))
  (Actor|DestroyActor))

(event EventBeginPlay
  (bind _returnvalue (Game|SpawnActorfromClass "/Game/02_Components/InventoryComponent/BP_ItemFound.BP_ItemFound_C" (Transformation|GetActorTransform) "AlwaysSpawn" self 0))
  (Variables|Default|SetFoundGlow _returnvalue))

(event EventTick
  (params (DeltaSeconds :type Float%20%28single-precision%29))
  (if (Variables|Default|GetIsFound)
    (Default|StartGlow (Variables|Default|GetFoundGlow))
    (Utilities|Time|SetTimerbyEvent (EventDispatchers|CreateEvent (Variables|Default|GetFoundGlow) :!event EndGlow) 0.5)
    (Variables|Default|SetIsFound false)
    (else
      (Variables|Default|SetIsFound false))))

(fn ConstructionScript)

(fn SetItemFound
  (Variables|Default|SetIsFound true))