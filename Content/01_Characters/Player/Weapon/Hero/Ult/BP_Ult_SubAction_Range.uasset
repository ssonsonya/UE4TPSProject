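; Range actor for the hero ultimate that finds non-player characters inside a sphere and marks them with cursor decals.
; Sphere overlaps gather valid targets for one second after BeginPlay, then the plane is hidden and sphere collision is disabled.
; A decal is spawned for each gathered character, and Tick moves it to follow that character's X/Y position by matching array index.
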(event OnComponentBeginOverlap(Sphere)
  (params (OverlappedComponent :type Primitive%20Component%20Object%20Reference) (OtherActor :type Actor%20Object%20Reference) (OtherComp :type Primitive%20Component%20Object%20Reference) (OtherBodyIndex :type Integer) (bFromSweep :type Boolean) (SweepResult :type Hit%20Result%20Structure%20%28by%20ref%29))
  (bind (_outhitted _outhittedactor _outhittedcharacter) (CallFunction|CheckHittedCharacter OtherActor (Variables|Default|GetHittedCharacters)))
  (if _outhitted
    (Utilities|IsValid _outhittedcharacter
      (:Is%20Valid
        (Utilities|Casting|CastToBP_Player _outhittedcharacter
          (:CastFailed
            (Utilities|Array|Add (Variables|Default|GetHittedCharacters) _outhittedcharacter)))))))

(event Custom|CheckHitted
  (Variables|Default|SetTargetingHitted true)
  (for _array_element (Variables|Default|GetHittedCharacters)
    (bind _returnvalue (Rendering|Decal|SpawnDecalatLocation "/Game/08_Assets/UIImage/M_Cursor_Inst.M_Cursor_Inst" "100.000000,100.000000,100.000000" (Math|Vector|MakeVector (.x (Transformation|GetActorLocation _array_element)) (.y (Transformation|GetActorLocation _array_element)) 0.0) "-90.000000,0.000000,0.000000" 0.0))
    (Utilities|Array|Add (Variables|Default|GetDecals) _returnvalue)))

(event EventBeginPlay
  (Utilities|FlowControl|Delay 1.0)
  (Rendering|SetVisibility (Variables|Default|GetPlane) false false)
  (Collision|SetCollisionEnabled (Variables|Default|GetSphere) "NoCollision")
  (CallFunction|CheckHitted))

(event EventTick
  (params (DeltaSeconds :type Float%20%28single-precision%29))
  (if (Variables|Default|GetTargetingHitted)
    (for (_array_element _array_index) (Variables|Default|GetDecals)
      (Transformation|SetWorldLocation _array_element (Math|Vector|MakeVector (.x (Transformation|GetActorLocation (Utilities|Array|Get(acopy) (Variables|Default|GetHittedCharacters) _array_index))) (.y (Transformation|GetActorLocation (Utilities|Array|Get(acopy) (Variables|Default|GetHittedCharacters) _array_index))) 0.0) false false))))

(fn ConstructionScript)